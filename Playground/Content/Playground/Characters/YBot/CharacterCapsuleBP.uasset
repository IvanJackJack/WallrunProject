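; YBot character Blueprint whose graph only draws debug vectors for movement and wallrunning.
; Each Tick, a sequence draws a velocity line scaled by speed, plus wallrun lines while WallrunComponent has a valid hit and is wallrunning.
; A shared helper draws each line from the capsule's location along a given direction.
; Hardcoded branches act as toggles, with the character forward and sideward axes switched off.
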(event `self.ReceiveTick`
  (params (DeltaSeconds :type "Float (single-precision)"))
  (bind _returnvalue (`self.GetVelocity`))
  (bind _wallruncomponent (`self.WallrunComponent`))
  (if true
    (`|ExecutionSequence`
      (:`then_0`
        (if false
          (`self.Debug Vector from Capsule` (`self.characterSideward`) 100.0 (struct :`G` 1.0 :`B` 0.009933 :`A` 1.0) 5.0)
          (`self.Debug Vector from Capsule` (`self.characterForward`) 100.0 (struct :`R` 1.0 :`G` 0.006161 :`A` 1.0) 5.0)))
      (:`then_1`
        (bind _returnvalue_2 (`WallrunComponent.HasValidHit` _wallruncomponent))
        (if (and _returnvalue_2 (`WallrunComponent.bIsWallrunning` _wallruncomponent))
          (`self.Debug Vector from Capsule` (0.0 0.0 0.0) 300.0 (struct :`G` 0.208052 :`B` 1.0 :`A` 1.0) 5.0)
          (`self.Debug Vector from Capsule` (0.0 0.0 0.0) 1.0 (struct :`R` 1.0 :`G` 0.367271 :`A` 1.0) 5.0)
          (`self.Debug Vector from Capsule` (0.0 0.0 0.0) 300.0 (struct :`G` 0.152268 :`B` 1.0 :`A` 1.0) 5.0)
          (`self.Debug Vector from Capsule` (`WallrunComponent.wallrunDirection` _wallruncomponent) 150.0 (struct :`G` 0.734243 :`B` 1.0 :`A` 1.0) 6.0)))
      (:`then_3`
        (if true
          (`self.Debug Vector from Capsule` (`KismetMathLibrary.Normal` _returnvalue) (* (`KismetMathLibrary.VSize` _returnvalue) 0.334) (struct :`R` 1.0 :`B` 0.966577 :`A` 1.0) 4.0))))))

(fn `Debug Vector from Capsule`
  (params (Direction :type "Vector Structure") (Length :type "Float (double-precision)") (Color :type "LinearColor Structure") (Thickness :type "Float (double-precision)"))
  (bind _returnvalue (`SceneComponent.K2_GetComponentLocation` (`self.Capsule`)))
  (`KismetSystemLibrary.DrawDebugLine` _returnvalue (+ _returnvalue (* Direction Length)) Color 0.0 Thickness))

(fn `UserConstructionScript`)